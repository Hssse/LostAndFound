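; Base instrument actor that the player can enter and leave through an Interact toggle.
; Entering blends the view to the instrument, disables character movement and enables input on the actor.
; Interacting again blends the view back to the character, restores walking and disables the actor's input.
; An empty completeChallenge event is declared with no logic.
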(event `/Game/Blueprints/Interactable.Interact`
  (if (`self.isInteracting`)
    (set `self.isInteracting` false)
    (`PlayerController.SetViewTargetWithBlend` (`GameplayStatics.GetPlayerController` 0) (`GameplayStatics.GetPlayerCharacter` 0) 2.0 "VTBlend_Linear" 0.0 false)
    (`CharacterMovementComponent.SetMovementMode` (`Character.CharacterMovement` (`GameplayStatics.GetPlayerCharacter` 0)) "MOVE_Walking" 0)
    (`self.DisableInput` (`GameplayStatics.GetPlayerController` 0))
    (else
      (set `self.isInteracting` true)
      (`PlayerController.SetViewTargetWithBlend` (`GameplayStatics.GetPlayerController` 0) self 2.0 "VTBlend_Linear" 0.0 false)
      (`CharacterMovementComponent.DisableMovement` (`Character.CharacterMovement` (`GameplayStatics.GetPlayerCharacter` 0)))
      (`self.EnableInput` (`GameplayStatics.GetPlayerController` 0)))))

(event `completeChallenge`)

(fn `UserConstructionScript`)