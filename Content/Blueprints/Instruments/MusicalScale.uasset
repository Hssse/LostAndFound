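; MusicalScale is an interactable crank puzzle where the player must rotate a handle at a target average speed.
; Interacting blends the view to the instrument and toggles player movement.
; While dragging, Tick converts mouse motion around the viewport center into angular deltas that turn the handle and set audio pitch from their running sum.
; Keeping the average delta within tolerance for TimeToHold calls the completion event, which is still empty.
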(event `rotateHandle`
  (`SceneComponent.K2_AddLocalRotation` (`self.centerPoint`) (`KismetMathLibrary.MakeRotator` (* (`self.curDelta`) -1.0)) false false))

(event `updateSound`
  (`AudioComponent.SetPitchMultiplier` (`self.Audio`) (/ (`self.DeltasSum`) (`self.targetDelta`))))

(event `checkDelta`
  (if (`self.isAverageDeltaInTargetRange`)
    (`KismetSystemLibrary.PrintString` (`KismetStringLibrary.Conv_DoubleToString` (`self.getAverageDelta`)))
    (if (> (- (`KismetSystemLibrary.GetGameTimeInSeconds`) (`self.startHoldTime`)) (`self.TimeToHold`))
      (`self.completeChallendge`))
    (else
      (set `self.startHoldTime` (`KismetSystemLibrary.GetGameTimeInSeconds`)))))

(event `completeChallendge`)

(event `self.ReceiveTick`
  (params (DeltaSeconds :type "Float (single-precision)"))
  (if (`self.isRotating`)
    (bind _returnvalue (`WidgetLayoutLibrary.GetMousePositionOnViewport`))
    (bind _deltarotation (`self.calcDeltaRotation` _returnvalue))
    (bind _output_get (set `self.curDelta` _deltarotation))
    (set `self.DeltasSum` (+ _output_get (`self.DeltasSum`)))
    (`self.rotateHandle`)
    (`self.updateSound`)
    (`self.checkDelta`)
    (set `self.prevMousePosition` _returnvalue)))

(event `self.HandleMesh.OnClicked`
  (params (TouchedComponent :type "PrimitiveComponent Object Reference") (ButtonPressed :type "Key Structure"))
  (if (`self.isInteracting`)
    (`self.startRotating`)))

(event `/Game/Blueprints/Interactable.Interact`
  (if (`self.isInteracting`)
    (set `self.isInteracting` false)
    (bind _aslaf_character (cast `/Game/Blueprints/Player/LAF_Character` (`GameplayStatics.GetPlayerPawn` 0)))
    (remove `/Game/Blueprints/Player/LAF_Character.onMouseReleased` _aslaf_character (`|CreateDelegate` :!event `StopRotating`))
    (`PlayerController.SetViewTargetWithBlend` (`GameplayStatics.GetPlayerController` 0) _aslaf_character 2.0 "VTBlend_Linear" 0.0 false)
    (`CharacterMovementComponent.SetMovementMode` (`Character.CharacterMovement` (`GameplayStatics.GetPlayerCharacter` 0)) "MOVE_Walking" 0)
    (else
      (set `self.isInteracting` true)
      (bind _aslaf_character_2 (cast `/Game/Blueprints/Player/LAF_Character` (`GameplayStatics.GetPlayerPawn` 0)))
      (add `/Game/Blueprints/Player/LAF_Character.onMouseReleased` _aslaf_character_2 (`|CreateDelegate` :!event `StopRotating`))
      (`PlayerController.SetViewTargetWithBlend` (`GameplayStatics.GetPlayerController` 0) self 2.0 "VTBlend_Linear" 0.0 false)
      (`CharacterMovementComponent.DisableMovement` (`Character.CharacterMovement` (`GameplayStatics.GetPlayerCharacter` 0))))))

(event `startRotating`
  (set `self.isRotating` true)
  (bind _returnvalue (`WidgetLayoutLibrary.GetMousePositionOnViewport`))
  (set `self.prevMousePosition` _returnvalue)
  (set `self.startRotatingTime` (`KismetSystemLibrary.GetGameTimeInSeconds`))
  (set `self.DeltasSum` 0.0))

(event `StopRotating`
  (set `self.isRotating` false))

(fn `calcDeltaRotation`
  (params (curPosition :type "Vector2D Structure"))
  (returns (deltaRotation :type "Float (double-precision)"))
  (return (.yaw (`KismetMathLibrary.NormalizedDeltaRotator` (`KismetMathLibrary.FindLookAtRotation` (`KismetMathLibrary.Conv_Vector2DToVector` (/ (`WidgetLayoutLibrary.GetViewportSize`) 2.0)) (`KismetMathLibrary.Conv_Vector2DToVector` (`local.curPosition`))) (`KismetMathLibrary.FindLookAtRotation` (`KismetMathLibrary.Conv_Vector2DToVector` (/ (`WidgetLayoutLibrary.GetViewportSize`) 2.0)) (`KismetMathLibrary.Conv_Vector2DToVector` (`self.prevMousePosition`)))))))

(fn `getAverageDelta`
  (returns (ReturnValue :type "Float (double-precision)"))
  (return (/ (`self.DeltasSum`) (- (`KismetSystemLibrary.GetGameTimeInSeconds`) (`self.startRotatingTime`)))))

(fn `isAverageDeltaInTargetRange`
  (returns (ReturnValue :type Boolean))
  (bind _returnvalue (`self.getAverageDelta`))
  (bind _targetdelta (`self.targetDelta`))
  (return (and (> _returnvalue (- _targetdelta (`self.deltaVariation`))) (< _returnvalue (+ _targetdelta (`self.deltaVariation`))))))

(fn `UserConstructionScript`)