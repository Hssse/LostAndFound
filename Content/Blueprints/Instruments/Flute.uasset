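; Flute instrument Blueprint that runs a note-sequence challenge played on the keyboard.
; Ten letter keys each send a note enum to pressKey, which only responds while Caps Lock is held.
; Correct notes advance an index through CorrectOrder and call CompleteChallenge at the end.
; A wrong note or releasing Caps Lock resets progress to the start.
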(event `Key|A`
  (params (Key :type "Key Structure"))
  (:`Pressed`
    (`self.pressKey` "NewEnumerator0")))

(event `self.ReceiveBeginPlay`
  (set `self.fluteKeys` (`|MakeArray` null null null null null null null null null null :!type "StaticMeshComponent Object Reference")))

(event `Key|S`
  (params (Key :type "Key Structure"))
  (:`Pressed`
    (`self.pressKey` "NewEnumerator1")))

(event `Key|D`
  (params (Key :type "Key Structure"))
  (:`Pressed`
    (`self.pressKey` "NewEnumerator2")))

(event `Key|E`
  (params (Key :type "Key Structure"))
  (:`Pressed`
    (`self.pressKey` "NewEnumerator3")))

(event `Key|F`
  (params (Key :type "Key Structure"))
  (:`Pressed`
    (`self.pressKey` "NewEnumerator4")))

(event `Key|G`
  (params (Key :type "Key Structure"))
  (:`Pressed`
    (`self.pressKey` "NewEnumerator5")))

(event `Key|H`
  (params (Key :type "Key Structure"))
  (:`Pressed`
    (`self.pressKey` "NewEnumerator6")))

(event `Key|J`
  (params (Key :type "Key Structure"))
  (:`Pressed`
    (`self.pressKey` "NewEnumerator7")))

(event `Key|K`
  (params (Key :type "Key Structure"))
  (:`Pressed`
    (`self.pressKey` "NewEnumerator8")))

(event `Key|L`
  (params (Key :type "Key Structure"))
  (:`Pressed`
    (`self.pressKey` "NewEnumerator9")))

(event `Key|CapsLock`
  (params (Key :type "Key Structure"))
  (:`Pressed`
    (set `self.isPlaying` true))
  (:`Released`
    (set `self.isPlaying` false)
    (set `self.currentIndex` 0)))

(event `pressKey`
  (params (NewParam :type "/Game/Blueprints/Instruments/FluteKeys Enum" :default "NewEnumerator0"))
  (if (`self.isPlaying`)
    (if (`|EnumEquality` NewParam (`|GetArrayItem` (`self.correctOrder`) (`self.currentIndex`)))
      (bind _output_get (set `self.currentIndex` (+ (`self.currentIndex`) 1)))
      (if (== _output_get (`KismetArrayLibrary.Array_Length` (`self.correctOrder`)))
        (`self.completeChallenge`))
      (else
        (set `self.currentIndex` 0)))))

(fn `UserConstructionScript`)