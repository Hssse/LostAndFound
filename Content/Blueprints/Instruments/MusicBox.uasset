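; Music box challenge where the player drags the handle around with the mouse at a target speed.
; Each tick, screen-space angle change around the projected center turns the handle and feeds a decaying sum used as speed.
; That speed bends the sound's pitch until it is within tolerance, where hold time builds; outside, it drains.
; Hold time swings the cap open and completes the challenge once past the threshold.
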(event `rotateHandleAndCap`
  (`SceneComponent.K2_AddLocalRotation` (`self.centerPoint`) (`KismetMathLibrary.MakeRotator` 0.0 (`self.curDelta`)) false false)
  (`SceneComponent.K2_SetRelativeRotation` (`self.BoxCap`) (`KismetMathLibrary.RLerp` (struct) (struct :`Pitch` 90.0) (`KismetMathLibrary.FClamp` (/ (`self.holdingTime`) (`self.TimeToHold`)))) false false))

(event `updateSound`
  (`AudioComponent.SetPitchMultiplier` (`self.CurSound`) (select `bool` (`self.isAverageDeltaInTargetRange`) :`false` (/ (`self.getAverageDelta`) (`self.targetDelta`)) :`true` 1.0)))

(event `checkDelta`
  (set `self.holdingTime` (`KismetMathLibrary.FMax` (+ (`self.holdingTime`) (* (`GameplayStatics.GetWorldDeltaSeconds`) (select `bool` (`self.isAverageDeltaInTargetRange`) :`false` -1.0 :`true` 1.0 :!type "Float (single-precision)")))))
  (if (> (`self.holdingTime`) (`self.TimeToHold`))
    (`/Engine/EditorBlueprintResources/StandardMacros.DoOnce` false
      (:`Completed`
        (`self.completeChallenge`)))))

(event `self.ReceiveTick`
  (params (DeltaSeconds :type "Float (single-precision)"))
  (if (`self.isCompleted`)
    _
    (elif (`self.isInteracting`)
      (if (`self.isRotating`)
        (bind _returnvalue (`WidgetLayoutLibrary.GetMousePositionOnViewport`))
        (bind _returnvalue_2 (* (/ _returnvalue (1920.0 1080.0)) (`WidgetLayoutLibrary.GetViewportSize`)))
        (bind _deltarotation (`self.calcDeltaRotation` _returnvalue_2))
        (bind _output_get (set `self.curDelta` _deltarotation))
        (set `self.DeltasSum` (`KismetMathLibrary.FMax` (- (+ _output_get (`self.DeltasSum`)) (* (`self.decreaseSpeed`) (`GameplayStatics.GetWorldDeltaSeconds`)))))
        (`self.rotateHandleAndCap`)
        (`self.updateSound`)
        (`self.checkDelta`)
        (set `self.prevMousePosition` _returnvalue_2)))))

(event `self.HandleMesh.OnClicked`
  (params (TouchedComponent :type "PrimitiveComponent Object Reference") (ButtonPressed :type "Key Structure"))
  (if (`self.isInteracting`)
    (`self.startRotating`)))

(event `StartRotating`
  (set `self.isRotating` true)
  (bind _returnvalue (`WidgetLayoutLibrary.GetMousePositionOnViewport`))
  (set `self.prevMousePosition` _returnvalue)
  (set `self.startRotatingTime` (`KismetSystemLibrary.GetGameTimeInSeconds`))
  (set `self.DeltasSum` 0.0)
  (`ActorComponent.Activate` (`self.CurSound`) true))

(event `StopRotating`
  (set `self.isRotating` false)
  (`ActorComponent.Deactivate` (`self.CurSound`)))

(event `/Game/Blueprints/Interactable.Interact`
  (bind _returnvalue (`GameplayStatics.GetPlayerController` 0))
  (`parent.Interact`)
  (if (not (`self.isCompleted`))
    (bind _aslaf_character (cast `/Game/Blueprints/Player/LAF_Character` (`GameplayStatics.GetPlayerCharacter` 0)))
    (if (`self.isInteracting`)
      (add `/Game/Blueprints/Player/LAF_Character.onMouseReleased` _aslaf_character (`|CreateDelegate` :!event `StopRotating`))
      (set `PlayerController.bShowMouseCursor` true _returnvalue)
      (else
        (remove `/Game/Blueprints/Player/LAF_Character.onMouseReleased` _aslaf_character (`|CreateDelegate` :!event `StopRotating`) :!label _label)
        (set `PlayerController.bShowMouseCursor` false _returnvalue)))))

(event `self.completeChallenge`
  (`self.StopRotating`)
  (`parent.completeChallenge`)
  (goto _label))

(fn `calcDeltaRotation`
  (params (curPosition :type "Vector2D Structure"))
  (returns (deltaRotation :type "Float (double-precision)"))
  (bind _screenposition (`GameplayStatics.ProjectWorldToScreen` (`GameplayStatics.GetPlayerController` 0) (`SceneComponent.K2_GetComponentLocation` (`self.centerPoint`))))
  (return (.yaw (`KismetMathLibrary.NormalizedDeltaRotator` (`KismetMathLibrary.FindLookAtRotation` (`KismetMathLibrary.Conv_Vector2DToVector` _screenposition) (`KismetMathLibrary.Conv_Vector2DToVector` (`local.curPosition`))) (`KismetMathLibrary.FindLookAtRotation` (`KismetMathLibrary.Conv_Vector2DToVector` _screenposition) (`KismetMathLibrary.Conv_Vector2DToVector` (`self.prevMousePosition`)))))))

(fn `getAverageDelta`
  (returns (ReturnValue :type "Float (double-precision)"))
  (return (`self.DeltasSum`)))

(fn `isAverageDeltaInTargetRange`
  (returns (ReturnValue :type Boolean))
  (bind _returnvalue (`self.getAverageDelta`))
  (bind _targetdelta (`self.targetDelta`))
  (return (and (> _returnvalue (- _targetdelta (`self.deltaVariation`))) (< _returnvalue (+ _targetdelta (`self.deltaVariation`))))))

(fn `UserConstructionScript`)