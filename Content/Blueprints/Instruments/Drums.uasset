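; Drum kit Blueprint for a sequence puzzle in which the player hits bass, drum and cymbals in the correct order.
; SpaceBar, Enter and CapsLock each register a hit and play a timeline that squishes the matching mesh's scale.
; On BeginPlay, a hint timeline triggers those same squish animations without registering hits.
; Hits advance an index through CorrectOrder, resetting on a mistake and calling CompleteChallenge at the end.
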(event `self.ReceiveBeginPlay`
  (`Timeline|hintTimeline` :!via `PlayFromStart`
    (:`bassHint`
      (`TimelineComponent.PlayFromStart` (`self.playBassTimeline`)))
    (:`drumHint`
      (`TimelineComponent.PlayFromStart` (`self.PlayDrumTimeline`)))
    (:`CymbalsHint`
      (`TimelineComponent.PlayFromStart` (`self.PlayCymbalsTimeline`)))))

(event `Key|SpaceBar`
  (params (Key :type "Key Structure"))
  ;[1 1 1] Play Drums
  (:`Pressed`
    (`self.playDrum` "NewEnumerator0")
    (bind (_direction _alpha) (`Timeline|playBassTimeline` :!via `PlayFromStart`)
      (:`Update`
        (`SceneComponent.SetRelativeScale3D` (`self.BassMesh`) (`KismetMathLibrary.VLerp` (1.0 1.0 1.0) (`self.bassSquishedScale`) _alpha))))))

(event `Key|Enter`
  (params (Key :type "Key Structure"))
  ;[1 1 1] Play Drums
  (:`Pressed`
    (`self.playDrum` "NewEnumerator1")
    (bind (_direction _alpha) (`Timeline|PlayDrumTimeline` :!via `PlayFromStart`)
      (:`Update`
        (`SceneComponent.SetRelativeScale3D` (`self.DrumMesh`) (`KismetMathLibrary.VLerp` (1.0 1.0 1.0) (`self.drumSquishedScale`) _alpha))))))

(event `Key|CapsLock`
  (params (Key :type "Key Structure"))
  ;[1 1 1] Play Drums
  (:`Pressed`
    (`self.playDrum` "NewEnumerator2")
    (bind (_direction _alpha) (`Timeline|PlayCymbalsTimeline` :!via `PlayFromStart`)
      (:`Update`
        (`SceneComponent.SetRelativeScale3D` (`self.Cymbals`) (`KismetMathLibrary.VLerp` (0.5 0.5 0.2) (`self.cymbalsSquishedScale`) _alpha))))))

(event `playDrum`
  (params (drumType :type "/Game/Blueprints/Instruments/DrumType Enum" :default "NewEnumerator0"))
  (if (`|EnumEquality` drumType (`|GetArrayItem` (`self.correctOrder`) (`self.currentIndex`)))
    (bind _output_get (set `self.currentIndex` (+ (`self.currentIndex`) 1)))
    (if (== _output_get (`KismetArrayLibrary.Array_Length` (`self.correctOrder`)))
      (`self.completeChallenge`))
    (else
      (set `self.currentIndex` 0))))

(fn `UserConstructionScript`)