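; Interactive piano puzzle where the player watches and hears each chord played note by note, then clicks the keys to repeat it.
; Input is blocked during previews; clicks are cursor-traced to key meshes, mapped to note enums, and answered with sound and material feedback.
; Completing a chord in any order advances the sequence, while a wrong key sounds higher-pitched and resets progress.
; Finishing all chords completes the inherited challenge.
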(event `self.ReceiveBeginPlay`
  ;[1 1 1] Comment
  (set `self.noteMeshes` (`|MakeArray` (`self.Note_C`) (`self.Note_C#`) (`self.Note_D`) (`self.Note_D#`) (`self.Note_E`) (`self.Note_F`) (`self.Note_F#`) (`self.Note_G`) (`self.Note_G#`) (`self.Note_A`) (`self.Note_A#`) (`self.NoteB`))))

(event `self.Interact`
  (bind _returnvalue (`GameplayStatics.GetPlayerController` 0))
  ;[1 1 1] Instrument
  (`parent.Interact`)
  (if (`self.isInteracting`)
    (set `PlayerController.bShowMouseCursor` true _returnvalue)
    (set `self.currentIndex` 0)
    (`self.viewNextChord`)
    (else
      (set `PlayerController.bShowMouseCursor` false _returnvalue))))

(event `self.completeChallenge`
  ;[1 1 1] Instrument
  (`parent.completeChallenge`))

(event `self.ReceiveActorOnClicked`
  (params (ButtonPressed :type "Key Structure"))
  ;[1 1 1] Press On Keys
  (if (and (`self.isInteracting`) (not (`self.isBlocked`)))
    (bind _asstatic_mesh_component (cast `StaticMeshComponent` (`.HitComponent` (`GameplayStatics.BreakHitResult` (`PlayerController.GetHitResultUnderCursorByChannel` (`GameplayStatics.GetPlayerController` 0) "TraceTypeQuery2" true)))))
    (`self.ToggleNote` _asstatic_mesh_component)))

(event `viewNextChord`
  (bind _output_notes (break `/Game/Blueprints/Instruments/PianoChord` (`|GetArrayItem` (`self.correctChords`) (`self.currentIndex`))))
  (bind _output_notes_2 (break `/Game/Blueprints/Instruments/PianoChord` (`|GetArrayItem` (`self.correctChords`) (`self.currentIndex`))))
  (bind _output (`|GetArrayItem` _output_notes_2 (`self.viewNoteIndex`)))
  (`self.resetPiano`)
  (set `self.viewNoteIndex` 0)
  (set `self.isBlocked` true)
  (if (== (`KismetArrayLibrary.Array_Length` (`self.correctChords`)) (`self.currentIndex`))
    (`self.completeChallenge`)
    (else
      (if (!= (`KismetArrayLibrary.Array_Length` _output_notes) (`self.viewNoteIndex`)) :!label _label
        (`self.lightUpNote` _output "NewEnumerator1")
        (`GameplayStatics.PlaySoundAtLocation` (`BlueprintMapLibrary.Map_Find` (`self.noteToSound`) _output) (`self.K2_GetActorLocation`) (struct) 1.0 1.0 0.0 null null null)
        (set `self.viewNoteIndex` (+ (`self.viewNoteIndex`) 1))
        (`KismetSystemLibrary.Delay` 0.5)
        (goto _label)
        (else
          (`self.resetPiano`)
          (set `self.isBlocked` false))))))

(event `lightUpNote`
  (params (Note :type "/Game/Blueprints/Instruments/PianoNotes Enum" :default "NewEnumerator0") (lightType :type "/Game/Blueprints/Instruments/PianoNoteLightUp Enum" :default "NewEnumerator0"))
  (`PrimitiveComponent.SetMaterial` (`|GetArrayItem` (`self.noteMeshes`) (`KismetMathLibrary.Conv_ByteToInt` Note)) 0 (select `/Game/Blueprints/Instruments/PianoNoteLightUp` lightType :`NewEnumerator0` "/Game/Assets/Materials/GreyMaterial.GreyMaterial" :`NewEnumerator1` "/Game/Assets/Materials/PreviewMaterial.PreviewMaterial" :`NewEnumerator2` "/Game/Assets/Materials/CorrectMaterial.CorrectMaterial" :`NewEnumerator3` "/Game/Assets/Materials/WrongMaterial.WrongMaterial" :!type "MaterialInterface Object Reference")))

(fn `getNoteByComponent`
  (params (NoteComponent :type "StaticMeshComponent Object Reference (by ref)"))
  (returns (Note :type "/Game/Blueprints/Instruments/PianoNotes Enum"))
  (return (cast `/Game/Blueprints/Instruments/PianoNotes` (`KismetMathLibrary.Conv_IntToByte` (`KismetArrayLibrary.Array_Find` (`self.noteMeshes`) NoteComponent)))))

(fn `isCorrectNotePlayed`
  (params (note :type "/Game/Blueprints/Instruments/PianoNotes Enum" :default "NewEnumerator0"))
  (returns (isCorrect :type Boolean))
  (bind _output_notes (break `/Game/Blueprints/Instruments/PianoChord` (`|GetArrayItem` (`self.correctChords`) (`self.currentIndex`))))
  (return (!= (`KismetArrayLibrary.Array_Find` _output_notes note) -1)))

(fn `resetPiano`
  (`KismetArrayLibrary.Array_Clear` (`self.pressedNotes`))
  (bind _enumvalue (foreach `/Game/Blueprints/Instruments/PianoNotes` false)
    (:`LoopBody`
      (`self.lightUpNote` _enumvalue))))

(fn `ToggleNote`
  (params (clickedNote :type "StaticMeshComponent Object Reference (by ref)"))
  (locals (localNote :type "/Game/Blueprints/Instruments/PianoNotes Enum" :default "NewEnumerator0"))
  (bind _localnote (`local.localNote`))
  (bind _note (`self.getNoteByComponent` clickedNote))
  (set `local.localNote` _note)
  (if (== (`KismetArrayLibrary.Array_Find` (`self.pressedNotes`) (`local.localNote`)) -1)
    (`KismetArrayLibrary.Array_AddUnique` (`self.pressedNotes`) (`local.localNote`))
    (bind _iscorrect (`self.isCorrectNotePlayed` _localnote))
    (`GameplayStatics.PlaySoundAtLocation` (`BlueprintMapLibrary.Map_Find` (`self.noteToSound`) _localnote) (`self.K2_GetActorLocation`) (struct) 1.0 (`KismetMathLibrary.SelectFloat` 1.0 3.0 _iscorrect) 0.0 null null null)
    (if _iscorrect
      (`self.lightUpNote` (`local.localNote`) "NewEnumerator2")
      (bind _iscorrect_2 (`self.verifyChord`))
      (if _iscorrect_2
        (set `self.currentIndex` (+ (`self.currentIndex`) 1))
        (`KismetSystemLibrary.K2_SetTimerDelegate` (`|CreateDelegate` :!event `viewNextChord`) 0.5))
      (else
        (set `self.currentIndex` 0)
        (`self.lightUpNote` (`local.localNote`) "NewEnumerator3")
        (`KismetSystemLibrary.K2_SetTimerDelegate` (`|CreateDelegate` :!event `viewNextChord`) 0.5)))))

(fn `UserConstructionScript`)

(fn `verifyChord`
  (returns (isCorrect :type Boolean))
  (locals (localIsCorrect :type Boolean :default true))
  (bind _output_notes (break `/Game/Blueprints/Instruments/PianoChord` (`|GetArrayItem` (`self.correctChords`) (`self.currentIndex`))))
  (bind _output_notes_2 (break `/Game/Blueprints/Instruments/PianoChord` (`|GetArrayItem` (`self.correctChords`) (`self.currentIndex`))))
  (set `local.localIsCorrect` (== (`KismetArrayLibrary.Array_Length` _output_notes_2) (`KismetArrayLibrary.Array_Length` (`self.pressedNotes`))))
  (for _array_element _output_notes
    (if (== (`KismetArrayLibrary.Array_Find` (`self.pressedNotes`) _array_element) -1)
      (set `local.localIsCorrect` false)))
  (return (`local.localIsCorrect`)))