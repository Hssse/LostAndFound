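; Double bass instrument puzzle in which the player clicks four strings in a set order to complete a challenge.
; Interact calls the parent logic, then shows the mouse cursor only while interacting.
; Each string mesh's click passes its enum value to PlayString, which compares it with the CorrectOrder array at CurrentIndex.
; A match advances the index until CompleteChallenge fires at the end, while a wrong string resets it to zero.
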(event `self.String_1_Mesh.OnClicked`
  (params (TouchedComponent :type "PrimitiveComponent Object Reference") (ButtonPressed :type "Key Structure"))
  ;[1 1 1] PlayStrings
  (`self.playString` "NewEnumerator0"))

(event `self.String_2_Mesh.OnClicked`
  (params (TouchedComponent :type "PrimitiveComponent Object Reference") (ButtonPressed :type "Key Structure"))
  ;[1 1 1] PlayStrings
  (`self.playString` "NewEnumerator1"))

(event `self.String_3_Mesh.OnClicked`
  (params (TouchedComponent :type "PrimitiveComponent Object Reference") (ButtonPressed :type "Key Structure"))
  ;[1 1 1] PlayStrings
  (`self.playString` "NewEnumerator2"))

(event `self.String_4_Mesh.OnClicked`
  (params (TouchedComponent :type "PrimitiveComponent Object Reference") (ButtonPressed :type "Key Structure"))
  ;[1 1 1] PlayStrings
  (`self.playString` "NewEnumerator3"))

(event `/Game/Blueprints/Interactable.Interact`
  (bind _returnvalue (`GameplayStatics.GetPlayerController` 0))
  (`parent.Interact`)
  (if (`self.isInteracting`)
    (set `PlayerController.bShowMouseCursor` true _returnvalue)
    (else
      (set `PlayerController.bShowMouseCursor` false _returnvalue))))

(event `playString`
  (params (string :type "/Game/Blueprints/Instruments/DoubleBassStrings Enum" :default "NewEnumerator0"))
  (if (`|EnumEquality` string (`|GetArrayItem` (`self.correctOrder`) (`self.currentIndex`)))
    (bind _output_get (set `self.currentIndex` (+ (`self.currentIndex`) 1)))
    (if (== _output_get (`KismetArrayLibrary.Array_Length` (`self.correctOrder`)))
      (`self.completeChallenge`))
    (else
      (set `self.currentIndex` 0))))

(fn `UserConstructionScript`)